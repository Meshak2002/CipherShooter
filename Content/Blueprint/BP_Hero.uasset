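; BP_Hero is the hero Blueprint, which plays an intro sound at its location on BeginPlay and switches between camera views.
; The SwitchCAM input drives a FlipFlop that alternates which of the FPSCAM and Camera components is active.
; The same toggle turns controller yaw rotation on for the FPSCAM view and off for the other camera.
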(event EventBeginPlay
  (|CallParentFunction)
  (Audio|PlaySoundatLocation "/Game/DevTV_Assets/GameDevTV/VoiceOvers/Intro.Intro" (Transformation|GetActorLocation) "0, 0, 0" 1.0 1.0 0.0 0 0 0 0))

(event Collision|EventActorBeginOverlap
  (params (OtherActor :type Actor%20Object%20Reference))
  (|CallParentFunction OtherActor) ; This node is disabled and will not be called.\nDrag off pins to build functionality.
)

(event EventTick
  (params (DeltaSeconds :type Float%20%28single-precision%29))
  (|CallParentFunction DeltaSeconds) ; This node is disabled and will not be called.\nDrag off pins to build functionality.
)

(event Input|ActionEvents|InputActionSwitchCAM
  (params (Key :type Key%20Structure :default "None"))
  (:Pressed
    (Utilities|FlowControl|FlipFlop
      (:A
        (Components|Activation|SetActive (Variables|Default|GetFPS%20CAM') true false)
        (Components|Activation|SetActive (Variables|Default|GetCamera) false false)
        (Variables|Default|SetbUseControllerRotationYaw true))
      (:B
        (Components|Activation|SetActive (Variables|Default|GetFPS%20CAM') false false)
        (Components|Activation|SetActive (Variables|Default|GetCamera) true false)
        (Variables|Default|SetbUseControllerRotationYaw false)))))

(fn ConstructionScript
  (|CallParentFunction))